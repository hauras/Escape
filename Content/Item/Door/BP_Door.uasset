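; BP_Door is a door actor that, once opened, becomes a portal moving the player to a target point.
; The OpenDoor event hides the door mesh, disables its collision, plays an unlock sound and enables query collision on a teleport trigger.
; When a BP_Player overlaps that trigger, it is teleported to the PortalTargetPoint actor's location with zero rotation.
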(event OnComponentBeginOverlap(TeleportTrigger)
  (params (OverlappedComponent :type Primitive%20Component%20Object%20Reference) (OtherActor :type Actor%20Object%20Reference) (OtherComp :type Primitive%20Component%20Object%20Reference) (OtherBodyIndex :type Integer) (bFromSweep :type Boolean) (SweepResult :type Hit%20Result%20Structure%20%28by%20ref%29))
  (bind _asbp_player (Utilities|Casting|CastToBP_Player OtherActor))
  (Transformation|Teleport _asbp_player (Transformation|GetActorLocation (Variables|Default|GetPortalTargetPoint)) "0, 0, 0"))

(event Collision|EventActorBeginOverlap
  (params (OtherActor :type Actor%20Object%20Reference)))

(event EventTick
  (params (DeltaSeconds :type Float%20%28single-precision%29)))

(event EventOpenDoor
  (bind _door (Variables|Default|GetDoor))
  (Rendering|SetVisibility _door false false)
  (Audio|PlaySoundatLocation "/Game/Assets/Sound/OpenDoor/UnLock.UnLock" "0, 0, 0" "0, 0, 0" 1.0 1.0 0.0 0 0 0 0)
  (Collision|SetCollisionEnabled _door "NoCollision")
  (Collision|SetCollisionEnabled (Variables|Default|GetTeleportTrigger) "QueryOnly"))

(fn ConstructionScript)